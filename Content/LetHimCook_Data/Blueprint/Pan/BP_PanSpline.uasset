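; BP_PanSpline moves a referenced actor, ActorToMove, along its spline once play begins.
; A timeline, rate-scaled by TimelineLength, drives a lerp over spline distance to set the actor's location each update.
; The actor's rotation follows the spline tangent, which is sampled in local space while location uses world space.
; The construction script snaps the actor to the first spline point.
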(event `self.ReceiveBeginPlay`
  (bind _spline (`self.Spline`))
  (bind _spline_2 (`self.Spline`))
  (bind _actortomove (`self.ActorToMove`))
  (`TimelineComponent.SetPlayRate` (`self.Timeline`) (/ 1.0 (`self.TimelineLength`)))
  (bind (_direction _alpha) (`Timeline|Timeline`)
    (:`Update`
      (bind _returnvalue (`KismetMathLibrary.Lerp` 0.0 (`SplineComponent.GetDistanceAlongSplineAtSplinePoint` _spline (- (`SplineComponent.GetNumberOfSplinePoints` _spline) 1)) _alpha))
      (`self.K2_SetActorLocation` _actortomove (`SplineComponent.GetLocationAtDistanceAlongSpline` _spline_2 _returnvalue "World") false false)
      (`self.K2_SetActorRotation` _actortomove (`KismetMathLibrary.Conv_VectorToRotator` (`SplineComponent.GetTangentAtDistanceAlongSpline` _spline_2 _returnvalue "Local")) false))))

(fn `UserConstructionScript`
  (`self.K2_SetActorLocation` (`self.ActorToMove`) (`SplineComponent.GetLocationAtSplinePoint` (`self.Spline`) 0 "World") false false))