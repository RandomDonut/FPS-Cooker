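; BP_PaneerPickup is an interactable ammo pickup that refills the player's paneer ammo, reported on screen as a pistol reload.
; Hover events swap the mesh's overlay material and enable or disable input on the pickup.
; Pressing the pick-item input while hovered sets BP_Player's paneer count to a fixed amount rather than adding to it.
; The pickup stays in the world after use.
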(event `self.On Hover`
  (params (IsHovering :type Boolean))
  (`MeshComponent.SetOverlayMaterial` (`self.PickupMesh`) "/Game/LetHimCook_Data/Blueprint/InteractionMat.InteractionMat")
  (`self.EnableInput` (`GameplayStatics.GetPlayerController` 0)))

(event `EnhancedInput|/Game/LetHimCook_Data/Blueprint/Inputs/IA_PickItem`
  (params (ActionValue :type Boolean) (ElapsedSeconds :type "Float (double-precision)") (TriggeredSeconds :type "Float (double-precision)") (InputAction :type "InputAction Object Reference" :default "/Game/LetHimCook_Data/Blueprint/Inputs/IA_PickItem.IA_PickItem"))
  (:`Started`
    (if (stale `self.On Hover` IsHovering)
      (bind _asbp_player (cast `/Game/LetHimCook_Data/Blueprint/BP_Player` (`GameplayStatics.GetPlayerPawn` 0)))
      (set `/Game/LetHimCook_Data/Blueprint/BP_Player.PaneerAmmoCount` 5 _asbp_player)
      (`KismetSystemLibrary.PrintString` "Pistol Reloaded!"))))

(event `self.On Hover End`
  (`MeshComponent.SetOverlayMaterial` (`self.PickupMesh`) "/Game/LetHimCook_Data/Blueprint/NonInteractionMat.NonInteractionMat")
  (`self.DisableInput` (`GameplayStatics.GetPlayerController` 0)))

(fn `UserConstructionScript`
  (`parent.UserConstructionScript`))