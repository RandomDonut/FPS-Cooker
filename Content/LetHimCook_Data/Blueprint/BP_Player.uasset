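; First-person player Blueprint handling Enhanced Input movement, camera look and weapon switching.
; Scroll inputs step through the Weapons array and swap the Weapon2 child actor's class.
; An overlap component sends hover messages to BPI_Interaction actors, while Tick starts walk or idle head-bob shakes based on velocity.
; A debug slow-motion input plays and reverses a timeline driving global time dilation, FOV and the High component's blend weight.
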(event `EnhancedInput|/Game/LetHimCook_Data/Blueprint/Inputs/IA_Camera`
  (params (ActionValue :type "Vector2D Structure") (ElapsedSeconds :type "Float (double-precision)") (TriggeredSeconds :type "Float (double-precision)") (InputAction :type "InputAction Object Reference" :default "/Game/LetHimCook_Data/Blueprint/Inputs/IA_Camera.IA_Camera"))
  ;[1 1 1] Add Camera Movement
  (:`Triggered`
    (`self.AddControllerYawInput` ActionValue_X)
    (`self.AddControllerPitchInput` ActionValue_Y)))

(event `self.ReceiveBeginPlay`
  ;[1 1 1] Add Mapping Context
  (bind _asplayer_controller (cast `PlayerController` (`self.GetController`)))
  (`/Engine/EditorBlueprintResources/StandardMacros.IsValid` _asplayer_controller
    (:`Is Valid`
      (`EnhancedInputSubsystemInterface.AddMappingContext` (pcsubsystem `EnhancedInputLocalPlayerSubsystem` _asplayer_controller) "/Game/LetHimCook_Data/Blueprint/Inputs/IMC_LetHimCook.IMC_LetHimCook" 0 (struct))
      ;[1 1 1] Set Initial Weapon
      (`ChildActorComponent.SetChildActorClass` (`self.Weapon2`) (`|GetArrayItem` (`self.Weapons`)))
      (`self.CharacterLoaded`)
      (set `PostProcessComponent.BlendWeight` 0.0 (`self.High`)))))

(event `EnhancedInput|/Game/LetHimCook_Data/Blueprint/Inputs/IA_ChangeWeaponNext`
  (params (ActionValue :type "Float (double-precision)") (ElapsedSeconds :type "Float (double-precision)") (TriggeredSeconds :type "Float (double-precision)") (InputAction :type "InputAction Object Reference" :default "/Game/LetHimCook_Data/Blueprint/Inputs/IA_ChangeWeaponNext.IA_ChangeWeaponNext"))
  (bind _returnvalue (+ (`KismetMathLibrary.FTrunc` ActionValue) (`self.Current Weapon Index`)))
  ;[1 1 1] Weapon Wheel Scroll
  (:`Triggered`
    (if (>= _returnvalue (`KismetArrayLibrary.Array_Length` (`self.Weapons`)))
      (set `self.Current Weapon Index` 0)
      (else
        (bind _output_get (set `self.Current Weapon Index` _returnvalue))))
    (`ChildActorComponent.SetChildActorClass` (`self.Weapon2`) (`|GetArrayItem` (`self.Weapons`) _output_get))))

(event `EnhancedInput|/Game/LetHimCook_Data/Blueprint/Inputs/IA_ChangeWeaponPrevious`
  (params (ActionValue :type "Float (double-precision)") (ElapsedSeconds :type "Float (double-precision)") (TriggeredSeconds :type "Float (double-precision)") (InputAction :type "InputAction Object Reference" :default "/Game/LetHimCook_Data/Blueprint/Inputs/IA_ChangeWeaponPrevious.IA_ChangeWeaponPrevious"))
  (bind _returnvalue (- (`self.Current Weapon Index`) (`KismetMathLibrary.FTrunc` ActionValue)))
  ;[1 1 1] Weapon Wheel Scroll
  (:`Triggered`
    (if (== _returnvalue -1)
      (set `self.Current Weapon Index` 1)
      (else
        (bind _output_get (set `self.Current Weapon Index` _returnvalue))))
    (`ChildActorComponent.SetChildActorClass` (`self.Weapon2`) (`|GetArrayItem` (`self.Weapons`) _output_get))))

(event `CharacterLoaded`
  ;[1 1 1] Unused Widget
  (`|CreateWidget` "/Game/LetHimCook_Data/Visuals/UI/WB_Crosshair.WB_Crosshair_C" (`GameplayStatics.GetPlayerController` 0)))

(event `EnhancedInput|/Game/LetHimCook_Data/Blueprint/Inputs/IA_Movement`
  (params (ActionValue :type "Vector2D Structure") (ElapsedSeconds :type "Float (double-precision)") (TriggeredSeconds :type "Float (double-precision)") (InputAction :type "InputAction Object Reference" :default "/Game/LetHimCook_Data/Blueprint/Inputs/IA_Movement.IA_Movement"))
  ;[1 1 1] Movement
  (:`Triggered`
    (`self.AddMovementInput` (`SceneComponent.GetRightVector` (`self.Camera`)) ActionValue_X)
    (`self.AddMovementInput` (`SceneComponent.GetForwardVector` (`self.Camera`)) ActionValue_Y)))

(event `self.ReceiveTick`
  (params (DeltaSeconds :type "Float (single-precision)"))
  (bind _returnvalue (`GameplayStatics.GetPlayerCameraManager` 0))
  ;[1 1 1] Camera Bobbing
  (if (> (`KismetMathLibrary.VSize` (`self.GetVelocity`)) 0.0)
    (`LegacyCameraShake.StartLegacyCameraShake` _returnvalue "/Game/LetHimCook_Data/Blueprint/CamershakePresets/BP_HeadBobWalk.BP_HeadBobWalk_C")
    (else
      (`LegacyCameraShake.StartLegacyCameraShake` _returnvalue "/Game/LetHimCook_Data/Blueprint/CamershakePresets/BP_HeadBobIdle.BP_HeadBobIdle_C"))))

(event `self.OverlapCheck.OnComponentBeginOverlap`
  (params (OverlappedComponent :type "PrimitiveComponent Object Reference") (OtherActor :type "Actor Object Reference") (OtherComp :type "PrimitiveComponent Object Reference") (OtherBodyIndex :type Integer) (bFromSweep :type Boolean) (SweepResult :type "HitResult Structure (by ref)"))
  ;[1 1 1] Overlap Check
  (if (`KismetSystemLibrary.DoesImplementInterface` OtherActor "/Game/LetHimCook_Data/Blueprint/BPI_Interaction.BPI_Interaction_C")
    (set `self.IsHovering` true)
    (message `/Game/LetHimCook_Data/Blueprint/BPI_Interaction.On Hover` OtherActor (`self.IsHovering`))))

(event `self.OverlapCheck.OnComponentEndOverlap`
  (params (OverlappedComponent :type "PrimitiveComponent Object Reference") (OtherActor :type "Actor Object Reference") (OtherComp :type "PrimitiveComponent Object Reference") (OtherBodyIndex :type Integer))
  ;[1 1 1] Overlap Check
  (message `/Game/LetHimCook_Data/Blueprint/BPI_Interaction.On Hover End` OtherActor)
  (set `self.IsHovering` false))

(event `EnhancedInput|/Game/LetHimCook_Data/Blueprint/Inputs/IA_SlowTimeDebug`
  (params (ActionValue :type Boolean) (ElapsedSeconds :type "Float (double-precision)") (TriggeredSeconds :type "Float (double-precision)") (InputAction :type "InputAction Object Reference" :default "/Game/LetHimCook_Data/Blueprint/Inputs/IA_SlowTimeDebug.IA_SlowTimeDebug"))
  ;[1 1 1] Debug Slow Motion
  (:`Triggered`
    (bind (_direction _slow_motion _fov_change _baked_curve) (`Timeline|FOV` :!label _label)
      (:`Update`
        (`GameplayStatics.SetGlobalTimeDilation` _slow_motion)
        (`CameraComponent.SetFieldOfView` (`self.Camera`) _fov_change)
        (set `PostProcessComponent.BlendWeight` _baked_curve (`self.High`)))))
  (:`Completed`
    (goto _label :!via `Reverse`)))

(fn `AmmoControl`
  (params (CurrentAmmo :type Integer :default 0)))

(fn `UserConstructionScript`)