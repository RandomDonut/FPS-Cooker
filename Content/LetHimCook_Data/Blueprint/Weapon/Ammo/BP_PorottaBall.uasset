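; BP_PorottaBall is a weapon ammo projectile that explodes visually a few seconds after it comes to a stop.
; When the projectile movement stops, the component deactivates and the mesh switches to physics simulation.
; After a fixed delay, it spawns an explosion particle at the mesh's current location and destroys itself, with no damage logic in this graph.
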(event `self.ReceiveBeginPlay`
  (`parent.ReceiveBeginPlay`))

(event `self.ProjectileMovement.OnProjectileStop`
  (params (ImpactResult :type "HitResult Structure (by ref)"))
  (`ActorComponent.Deactivate` (`self.ProjectileMovement`))
  (`PrimitiveComponent.SetSimulatePhysics` (`self.ProjectileMesh`) true)
  (`KismetSystemLibrary.Delay` 5.0)
  (`GameplayStatics.SpawnEmitterAtLocation` "/Game/StarterContent/Particles/P_Explosion.P_Explosion" (`SceneComponent.K2_GetComponentLocation` (`self.ProjectileMesh`)))
  (`self.K2_DestroyActor`))

(fn `UserConstructionScript`
  (`parent.UserConstructionScript`))