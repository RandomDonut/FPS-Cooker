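; BP_RPG is the player's rocket launcher weapon, firing projectiles from its Muzzle on the shoot input.
; Each shot checks and decrements the RPG ammo count stored on BP_Player and plays a heavy camera shake.
; Equipping runs on BeginPlay and creates a crosshair widget, with no viewport add here.
; Every Tick it predicts the projectile arc from muzzle direction and ammo speed, spawning a BP_PathActor at each path point.
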(event `WeaponFired`
  ;[1 1 1] Reduce Ammo
  (bind _output_get (set `/Game/LetHimCook_Data/Blueprint/BP_Player.RPGAmmoCount` (- (`/Game/LetHimCook_Data/Blueprint/BP_Player.RPGAmmoCount` (stale `self.ReceiveBeginPlay` _asbp_player)) 1) (stale `self.ReceiveBeginPlay` _asbp_player)))
  (`KismetSystemLibrary.PrintString` (`KismetStringLibrary.Conv_IntToString` _output_get)))

(event `self.ReceiveBeginPlay`
  ;[1 1 1] Weapon Equip
  (`parent.ReceiveBeginPlay`)
  (`self.OnWeaponEquip`)
  (bind _asbp_player (cast `/Game/LetHimCook_Data/Blueprint/BP_Player` (`GameplayStatics.GetPlayerPawn` 0))))

(event `EnhancedInput|/Game/LetHimCook_Data/Blueprint/Inputs/IA_Shoot`
  (params (ActionValue :type "Float (double-precision)") (ElapsedSeconds :type "Float (double-precision)") (TriggeredSeconds :type "Float (double-precision)") (InputAction :type "InputAction Object Reference" :default "/Game/LetHimCook_Data/Blueprint/Inputs/IA_Shoot.IA_Shoot"))
  (bind (_returnvalue_location _returnvalue_rotation) (`KismetMathLibrary.BreakTransform` (`SceneComponent.K2_GetComponentToWorld` (`self.Muzzle`))))
  ;[1 1 1] Fire Weapon
  (:`Started`
    (bind _output_get (set `self.IsWeaponEmpty` (== (`/Game/LetHimCook_Data/Blueprint/BP_Player.RPGAmmoCount` (stale `self.ReceiveBeginPlay` _asbp_player)) 0)))
    (if _output_get
      (`KismetSystemLibrary.PrintString` "Out of RPG Ammo" true true (struct :`R` 1.0 :`A` 1.0))
      (else
        (`|SpawnActorFromClass` (`self.AmmoProjectileClass`) (`KismetMathLibrary.MakeTransform` _returnvalue_location _returnvalue_rotation) "Undefined" "MultiplyWithRoot" null null)
        (`self.WeaponFired`)
        (`LegacyCameraShake.StartLegacyCameraShake` (`GameplayStatics.GetPlayerCameraManager` 0) "/Game/LetHimCook_Data/Blueprint/CamershakePresets/BP_ShootHeavy.BP_ShootHeavy_C")))))

(event `OnWeaponEquip`
  (`|CreateWidget` (`self.WeaponCrosshairWidget`) (`GameplayStatics.GetPlayerController` 0)))

(event `self.ReceiveTick`
  (params (DeltaSeconds :type "Float (single-precision)"))
  (bind _muzzle (`self.Muzzle`))
  (bind _predictresult (`GameplayStatics.Blueprint_PredictProjectilePath_Advanced` (make `PredictProjectilePathParams` (`SceneComponent.K2_GetComponentLocation` _muzzle) (* (`SceneComponent.GetForwardVector` _muzzle) (`self.AmmoSpeed`)) true 0.0 1.0 true "ECC_Visibility" _ _ 50.0)))
  (for _array_element (break `PredictProjectilePathResult` _predictresult)
    (`|SpawnActorFromClass` "/Game/LetHimCook_Data/Blueprint/Weapon/ProjectilePrediction/BP_PathActor.BP_PathActor_C" (`KismetMathLibrary.MakeTransform` (break `PredictProjectilePathPointData` _array_element) (`SceneComponent.K2_GetComponentRotation` (`self.Muzzle`))) "Undefined" "MultiplyWithRoot" null null)))

(fn `UserConstructionScript`
  (`parent.UserConstructionScript`))